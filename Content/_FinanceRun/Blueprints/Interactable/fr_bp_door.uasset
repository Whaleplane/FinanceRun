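; Interactable door for the Finance Run game that moves the player on to the next room.
; On InteractEvent it checks the current level name and normally opens the level named by its NextRoom variable.
; In room 10 it instead creates a retirement popup widget and adds it to the viewport, without changing level.
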(event EventBeginPlay)

(event Collision|EventActorBeginOverlap
  (params (OtherActor :type Actor%20Object%20Reference))
  (|CallParentFunction OtherActor) ; This node is disabled and will not be called.\nDrag off pins to build functionality.
)

(event EventTick
  (params (DeltaSeconds :type Float%20%28single-precision%29)))

(event EventInteractEvent
  (bind _returnvalue (Game|GetCurrentLevelName true))
  (if (Utilities|Enum|Equal(Enum) _returnvalue "fr_m_room10")
    (bind _returnvalue_2 (UserInterface|CreateWidget "/Game/_FinanceRun/UI/fr_w_retirementPopup1.fr_w_retirementPopup1_C"))
    (UserInterface|Viewport|AddtoViewport _returnvalue_2 0)
    (else
      (Game|OpenLevel(byName) (Variables|Default|GetnextRoom)))))

(fn ConstructionScript
  (|CallParentFunction))