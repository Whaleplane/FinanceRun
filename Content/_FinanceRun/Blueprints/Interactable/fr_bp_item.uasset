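; Collectible item for FinanceRun that boosts one random player stat when its interact event fires.
; InteractEvent picks at random among Knowledge, Preparation and Skill and calls the matching add function on the player character.
; All three branches then share the same feedback, a particle effect at the item's location and a 2D pickup sound.
; Overlap handling and construction defer entirely to the parent class.
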(event EventInteractEvent
  (bind _returnvalue (Game|GetPlayerCharacter 0))
  (bind _asfr_bp_player_character (Utilities|Casting|CastTofr_bp_playerCharacter _returnvalue))
  ;[1 1 1] Increment a random stat
  (switch int (Math|Random|RandomInteger 3)
    (:0
      (Default|AddKnowledge _asfr_bp_player_character))
    (:1
      (Default|AddPreparation _asfr_bp_player_character))
    (:2
      (Default|AddSkill _asfr_bp_player_character)))
  (Niagara|SpawnSystematLocation "/Game/_FinanceRun/Particles/fr_fx_item.fr_fx_item" (Transformation|GetActorLocation))
  (Audio|PlaySound2D "/Game/_FinanceRun/Audio/fr_cue_getItem.fr_cue_getItem" 1.0 1.0 0.0 0 0))

(event Collision|EventActorBeginOverlap
  (params (OtherActor :type Actor%20Object%20Reference))
  (|CallParentFunction OtherActor))

(fn ConstructionScript
  (|CallParentFunction))