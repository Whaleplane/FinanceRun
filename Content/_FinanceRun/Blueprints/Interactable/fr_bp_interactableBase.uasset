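; Base interactable actor that fires an overridable interact event when the player character overlaps it.
; A DoOnce gate blocks repeat triggers, and the player reference is stored before the empty InteractEvent runs for child Blueprints to fill in.
; It then either destroys itself when DeleteOnInteract is set or re-arms the gate after a short delay.
; Overlaps by other actors re-arm the gate immediately.
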(event Custom|interactEvent
  ;[1 1 1] Interact event, add code for children here
)

(event Custom|resetOverlap
  ;[1 1 1] Collision with player, play interact event and delete if boolean is true
  (Utilities|FlowControl|DoOnce false) ; enters at Reset
)

(event Collision|EventActorBeginOverlap
  (params (OtherActor :type Actor%20Object%20Reference))
  ;[1 1 1] Collision with player, play interact event and delete if boolean is true
  (Utilities|FlowControl|DoOnce false
    (:Completed
      (bind _asfr_bp_player_character (Utilities|Casting|CastTofr_bp_playerCharacter OtherActor)
        (:then
          (Variables|Default|SetprPlayer _asfr_bp_player_character)
          (CallFunction|InteractEvent)
          (if (Variables|Default|GetdeleteOnInteract)
            (CallFunction|ResetOverlap)
            (Actor|DestroyActor)
            (else
              (Utilities|FlowControl|Delay 0.6)
              (CallFunction|ResetOverlap :!label _label))))
        (:CastFailed
          (goto _label))))))

(fn ConstructionScript)