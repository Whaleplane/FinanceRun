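; Enemy character Blueprint for FinanceRun that feeds its AI controller's Blackboard for behavior logic.
; On BeginPlay it writes its starting location, wander radius and target distance to Blackboard keys.
; AI Perception updates set the target actor key to the player character, or clear it for any other actor.
; The update handler checks only the actor's class, not whether it was successfully sensed.
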(event OnTargetPerceptionUpdated(AIPerception)
  (params (Actor :type Actor%20Object%20Reference) (Stimulus :type AI%20Stimulus%20Structure))
  (bind _self self)
  (bind _bb_targetactor (Variables|Default|GetBB_TargetActor))
  (bind _returnvalue (AI|GetAIController _self))
  (bind _returnvalue_2 (AI|GetBlackboard _returnvalue))
  ;[1 1 1] Set target actor to player if perceived, set to null if not perceived
  (bind _asfr_bp_player_character (Utilities|Casting|CastTofr_bp_playerCharacter Actor)
    (:then
      (AI|Components|Blackboard|SetValueasObject _returnvalue_2 _bb_targetactor _asfr_bp_player_character))
    (:CastFailed
      (AI|Components|Blackboard|SetValueasObject _returnvalue_2 _bb_targetactor 0))))

(event EventBeginPlay
  (CallFunction|SetBlackboardKeys))

(fn ConstructionScript)

(fn SetBlackboardKeys
  (bind _self self)
  (bind _returnvalue (AI|GetAIController _self))
  (bind _returnvalue_2 (AI|GetBlackboard _returnvalue))
  ;[1 1 1] Set both initial blackboard keys
  (AI|Components|Blackboard|SetValueasVector _returnvalue_2 (LocalVariables|GetBB_InitialPosition) (Transformation|GetActorLocation))
  (AI|Components|Blackboard|SetValueasFloat _returnvalue_2 (LocalVariables|GetBB_WanderRadius) (Variables|Default|GetwanderRadius))
  (AI|Components|Blackboard|SetValueasFloat _returnvalue_2 (LocalVariables|GetBB_TargetDistance) (Variables|Default|GettargetDistance)))