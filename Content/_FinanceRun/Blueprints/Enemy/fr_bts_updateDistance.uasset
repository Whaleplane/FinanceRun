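; Behavior tree service for enemy AI that keeps the DistanceToTarget blackboard value current.
; On each tick it casts TargetActor to the player character and writes the distance from the controlled pawn to it.
; When that cast fails, it writes CombatRange plus a small margin, so a missing target always reads as out of combat range.
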(event EventReceiveTickAI
  (params (OwnerController :type AI%20Controller%20Object%20Reference) (ControlledPawn :type Pawn%20Object%20Reference) (DeltaSeconds :type Float%20%28single-precision%29))
  (bind _asfr_bp_player_character (Utilities|Casting|CastTofr_bp_playerCharacter (Class|BTFunctionLibrary|GetBlackboardValueasObject (Variables|Default|GetTargetActor)))
    (:then
      ;[1 1 1] Set distance to target
      (Class|BTFunctionLibrary|SetBlackboardValueasFloat (Variables|Default|GetdistanceToTarget) (Math|Vector|Distance(Vector) (Transformation|GetActorLocation ControlledPawn) (Transformation|GetActorLocation _asfr_bp_player_character))))
    (:CastFailed
      ;[1 1 1] Make sure target distance is always over range if there is no target
      (Class|BTFunctionLibrary|SetBlackboardValueasFloat (Variables|Default|GetdistanceToTarget) (+ (Class|BTFunctionLibrary|GetBlackboardValueasFloat (Variables|Default|GetcombatRange)) 1.0)))))