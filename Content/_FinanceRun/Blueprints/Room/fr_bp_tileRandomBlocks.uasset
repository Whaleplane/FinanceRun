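; Room tile actor that randomizes its layout at BeginPlay by removing pieces from four quarters, each made of a base block, height block and item.
; Weighted random bools for base, height and item feed one shared decision event per quarter, where true means destroy.
; Removing a base also removes its height block and possibly its item; otherwise only the height block can be removed.
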(event Custom|quarterDecision
  (params (base :type Boolean) (height :type Boolean) (item :type Boolean) (baseBlock :type Static%20Mesh%20Component%20Object%20Reference) (heightBlock :type Static%20Mesh%20Component%20Object%20Reference) (ItemActor :type Child%20Actor%20Component%20Object%20Reference))
  ;[1 1 1] Decision setup for each quarter
  (if base
    (Components|DestroyComponent baseBlock) ; Destroy base
    (if item
      (Components|DestroyComponent ItemActor) ; Destroy item
    )
    (Components|DestroyComponent heightBlock :!label _label) ; Destroy height
    (elif height
      (goto _label))))

(event EventBeginPlay
  (bind _weightitem (Variables|Default|GetweightItem))
  (bind _weightbase (Variables|Default|GetweightBase))
  (bind _weightheight (Variables|Default|GetweightHeight))
  (bind _returnvalue (Math|Random|RandomBoolwithWeight _weightheight))
  (bind _returnvalue_2 (Math|Random|RandomBoolwithWeight _weightitem))
  (bind _returnvalue_3 (Math|Random|RandomBoolwithWeight _weightbase))
  ;[1 1 1] Fire events for all four sets of blocks
  (|CallParentFunction)
  (CallFunction|QuarterDecision _returnvalue_3 _returnvalue _returnvalue_2 (Variables|Default|Getblock1) (Variables|Default|Getblock1h) (Variables|Default|Getitem1))
  (CallFunction|QuarterDecision _returnvalue_3 _returnvalue _returnvalue_2 (Variables|Default|Getblock2) (Variables|Default|Getblock2h) (Variables|Default|Getitem2))
  (CallFunction|QuarterDecision _returnvalue_3 _returnvalue _returnvalue_2 (Variables|Default|Getblock3) (Variables|Default|Getblock3h) (Variables|Default|Getitem3))
  (CallFunction|QuarterDecision _returnvalue_3 _returnvalue _returnvalue_2 (Variables|Default|Getblock4) (Variables|Default|Getblock4h) (Variables|Default|Getitem4)))

(event Collision|EventActorBeginOverlap
  (params (OtherActor :type Actor%20Object%20Reference))
  (|CallParentFunction OtherActor) ; This node is disabled and will not be called.\nDrag off pins to build functionality.
)

(event EventTick
  (params (DeltaSeconds :type Float%20%28single-precision%29))
  (|CallParentFunction DeltaSeconds) ; This node is disabled and will not be called.\nDrag off pins to build functionality.
)

(fn ConstructionScript
  (|CallParentFunction))