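; Core character Blueprint for FinanceRun that opens the main menu and manages video quality settings.
; On BeginPlay it adds the menu widget, shows the mouse cursor and reapplies the saved quality tier, defaulting to medium.
; Low, Medium and High events set scalability through console commands and save the chosen tier.
; SaveData and LoadData helpers persist values through EasySaveObject actors found in the level.
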(event Custom|Low%20Settings
  ;[1 1 1] Set and save video settings
  (Development|ExecuteConsoleCommand "r.PostProcessAAQuality 0" 0)
  (Development|ExecuteConsoleCommand "sg.PostProcessQuality 1" 0)
  (Development|ExecuteConsoleCommand "sg.ShadowQuality 1" 0)
  (Development|ExecuteConsoleCommand "sg.TextureQuality 1" 0)
  (CallFunction|SaveData "sQuality" "0"))

(event Custom|Medium%20Settings
  ;[1 1 1] Set and save video settings
  (Development|ExecuteConsoleCommand "r.PostProcessAAQuality 3" 0)
  (Development|ExecuteConsoleCommand "sg.PostProcessQuality 2" 0)
  (Development|ExecuteConsoleCommand "sg.ShadowQuality 2" 0)
  (Development|ExecuteConsoleCommand "sg.TextureQuality 2" 0)
  (CallFunction|SaveData "sQuality" "1"))

(event Custom|High%20Settings
  ;[1 1 1] Set and save video settings
  (Development|ExecuteConsoleCommand "r.PostProcessAAQuality 6" 0)
  (Development|ExecuteConsoleCommand "sg.PostProcessQuality 3" 0)
  (Development|ExecuteConsoleCommand "sg.ShadowQuality 3" 0)
  (Development|ExecuteConsoleCommand "sg.TextureQuality 3" 0)
  (CallFunction|SaveData "sQuality" "2"))

(event EventBeginPlay
  ;[1 1 1] Add main menu to viewport
  (bind _returnvalue (UserInterface|CreateWidget "/Game/_FinanceRun/UI/fr_w_mainMenu.fr_w_mainMenu_C"))
  (UserInterface|Viewport|AddtoViewport _returnvalue 0)
  (Variables|/Script/Engine.PlayerController|SetbShowMouseCursor (Game|GetPlayerController 0) true)
  ;[1 1 1] Load and set video quality settings
  (bind _returnvalue_2 (SaveGame|DoesSaveGameExist "sQuality"))
  (if _returnvalue_2
    (bind _keyvalue (CallFunction|LoadData "sQuality"))
    (switch int (Math|Float|Truncate _keyvalue)
      (:0
        (CallFunction|LowSettings))
      (:1
        (CallFunction|MediumSettings))
      (:2
        (CallFunction|HighSettings)))
    (else
      (CallFunction|MediumSettings))))

(fn ConstructionScript)

(fn SaveData
  (params (KeyName :type String) (KeyValue :type Text))
  ;[1 1 1] Save a value using EasySaveObject
  (bind _outactors (Actor|GetAllActorsOfClass "/Game/EasySave/easySaveObject.easySaveObject_C"))
  (for _array_element _outactors
    (bind _aseasy_save_object (Utilities|Casting|CastToeasySaveObject _array_element))
    (Default|EasySaveValue :self _aseasy_save_object :keyName KeyName :keyType "NewEnumerator1" :keyValue KeyValue)))

(fn LoadData
  (params (KeyName :type String))
  (bind _outactors (Actor|GetAllActorsOfClass "/Game/EasySave/easySaveObject.easySaveObject_C"))
  (for _array_element _outactors
    (bind _aseasy_save_object (Utilities|Casting|CastToeasySaveObject _array_element))
    (bind _valueasfloat (Default|EasyLoadValue _aseasy_save_object KeyName "NewEnumerator1" false))
    (return _valueasfloat)))