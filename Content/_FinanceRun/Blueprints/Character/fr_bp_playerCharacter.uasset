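; Player character for a finance game with a cursor-to-world marker, carrying money, salary and three stats across levels.
; BeginPlay picks a random job in the first room; later levels reload saved values, pay salary and apply saved vehicle and education adjustments.
; SaveData and LoadData persist values by key through EasySaveObject actors.
; StartCombat locks movement, faces the enemy and shows the combat HUD until FinishCombat restores control.
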(event Custom|AddMoney
  (params (moneyIn :type Float%20%28single-precision%29))
  ;[1 1 1] Add Money
  (Variables|Default|Setmoney (+ (Variables|Default|Getmoney) moneyIn))
  ;[1 1 1] Add to the earned subtotal
  (Variables|Default|SetearnedSubtotal (+ (Variables|Default|GetearnedSubtotal) moneyIn))
  ;[1 1 1] Resave money after modification
  (CallFunction|SaveData "pMoney" (Utilities|Text|ToText(Float) (Variables|Default|Getmoney) "HalfToEven" false false 1 324 2 2)))

(event Custom|RemoveMoney
  (params (MoneyIn :type Float%20%28single-precision%29))
  ;[1 1 1] Remove Money
  (Variables|Default|Setmoney (- (Variables|Default|Getmoney) MoneyIn))
  ;[1 1 1] Resave money after modification
  (CallFunction|SaveData "pMoney" (Utilities|Text|ToText(Float) (Variables|Default|Getmoney) "HalfToEven" false false 1 324 2 2)))

(event Custom|Face%20Enemy
  ;[1 1 1] Face Enemy (called from tick if in combat)
  (Transformation|SetActorRotation (Math|Rotator|FindLookatRotation (Transformation|GetActorLocation) (Transformation|GetActorLocation (Variables|Default|GetenemyToFace)))))

(event Custom|AddKnowledge
  ;[1 1 1] Increment and save stats
  (bind _result (Math|Integer|IncrementInt (Variables|Default|GetstatKnowledge))
    (:%20%20
      (CallFunction|SaveData "pKnowledge" (Utilities|Text|ToText(Integer) _result)))))

(event Custom|AddSkill
  ;[1 1 1] Increment and save stats
  (bind _result (Math|Integer|IncrementInt (Variables|Default|GetstatSkill))
    (:%20%20
      (CallFunction|SaveData "pSkill" (Utilities|Text|ToText(Integer) _result)))))

(event Custom|AddPreparation
  ;[1 1 1] Increment and save stats
  (bind _result (Math|Integer|IncrementInt (Variables|Default|GetstatPreparation))
    (:%20%20
      (CallFunction|SaveData "pPreparation" (Utilities|Text|ToText(Integer) _result)))))

(event Custom|Set%20Random%20Job
  ;[1 1 1] Select random job, set/save money and salary
  (bind _outrownames (DataTable|GetDataTableRowNames "/Game/_FinanceRun/Data/fr_data_jobs.fr_data_jobs"))
  (CallFunction|SaveData "pJobIndex" (Utilities|Text|ToText(Integer) (Math|Random|RandomInteger (Utilities|Array|Length _outrownames))))
  (bind _returnvalue (Utilities|GetDataTableRow "/Game/_FinanceRun/Data/fr_data_jobs.fr_data_jobs" (Utilities|Array|Get(acopy) _outrownames (Math|Random|RandomInteger (Utilities|Array|Length _outrownames))))
    (:then
      (bind _output_get (Variables|Default|Setmoney (/ (.SalaryBase (Utilities|Struct|Breakfr_struct_jobRows _returnvalue)) 1e+01)))
      (bind _output_get_2 (Variables|Default|Setsalary (/ (.SalaryBase (Utilities|Struct|Breakfr_struct_jobRows _returnvalue)) 1e+01)))
      (CallFunction|SaveData "pMoney" (Utilities|Text|ToText(Float) _output_get "HalfToEven" false false 1 324 0 2))
      (CallFunction|SaveData "pSalary" (Utilities|Text|ToText(Float) _output_get_2 "HalfToEven" false false 1 324 0 2))
      (switch int (.StatBonusIndex (Utilities|Struct|Breakfr_struct_jobRows _returnvalue))
        (:0
          (Variables|Default|SetstatKnowledge 5))
        (:1
          (Variables|Default|SetstatPreparation 5))
        (:2
          (Variables|Default|SetstatSkill 5))))))

(event EventBeginPlay
  ;[1 1 1] Create and add the HUD
  (bind _returnvalue (UserInterface|CreateWidget "/Game/_FinanceRun/UI/fr_w_hud.fr_w_hud_C"))
  (UserInterface|Viewport|AddtoViewport _returnvalue 0)
  ;[1 1 1] Load, add, and resave money, then load job index
  (bind _returnvalue_2 (Game|GetCurrentLevelName true))
  (if (Utilities|Enum|Equal(Enum) _returnvalue_2 "fr_m_room01")
    (Variables|Default|SetonFirstRoom true)
    (CallFunction|SetRandomJob)
    (else
      (bind _keyvalue (CallFunction|LoadData "pMoney"))
      (Variables|Default|Setmoney _keyvalue)
      (bind _keyvalue_2 (CallFunction|LoadData "pSalary"))
      (Variables|Default|Setsalary _keyvalue_2)
      (CallFunction|AddMoney _keyvalue_2)
      (bind _keyvalue_3 (CallFunction|LoadData "pJobIndex"))
      (Variables|Default|SetjobIndex (Math|Float|Truncate _keyvalue_3))))
  ;[1 1 1] Load and spend vehicle payment
  (if (Variables|Default|GetonFirstRoom)
    (CallFunction|SaveData "vPayment" "0")
    (else
      (bind _keyvalue_4 (CallFunction|LoadData "vPayment")) ; Saved in fr_w_vehiclePopup3
      (CallFunction|RemoveMoney _keyvalue_4)))
  ;[1 1 1] Load and set PREPARATION stat
  (if (Variables|Default|GetonFirstRoom)
    (CallFunction|SaveData "pPreparation" (Utilities|Text|ToText(Integer) (Variables|Default|GetstatKnowledge)))
    (else
      (bind _keyvalue_5 (CallFunction|LoadData "pPreparation")) ; Saved in fr_w_vehiclePopup3
      (Variables|Default|SetstatPreparation (Math|Float|Truncate _keyvalue_5))))
  ;[1 1 1] Load and set KNOWLEDGE stat
  (if (Variables|Default|GetonFirstRoom)
    (CallFunction|SaveData "pKnowledge" (Utilities|Text|ToText(Integer) (Variables|Default|GetstatPreparation)))
    (else
      (bind _keyvalue_6 (CallFunction|LoadData "pKnowledge")) ; Saved in fr_w_vehiclePopup3
      (Variables|Default|SetstatKnowledge (Math|Float|Truncate _keyvalue_6))))
  ;[1 1 1] Load and set SKILL stat
  (if (Variables|Default|GetonFirstRoom)
    (CallFunction|SaveData "pSkill" (Utilities|Text|ToText(Integer) (Variables|Default|GetstatSkill)))
    (else
      (bind _keyvalue_7 (CallFunction|LoadData "pSkill")) ; Saved in fr_w_vehiclePopup3
      (Variables|Default|SetstatSkill (Math|Float|Truncate _keyvalue_7))))
  ;[1 1 1] Load and spend education payment
  (if (Variables|Default|GetonFirstRoom)
    (CallFunction|SaveData "ePayment" "0")
    (else
      (bind _keyvalue_8 (CallFunction|LoadData "ePayment"))
      (CallFunction|RemoveMoney _keyvalue_8)))
  ;[1 1 1] Load and add education salary increase
  (if (Variables|Default|GetonFirstRoom)
    (CallFunction|SaveData "eIncrease" "0")
    (else
      (bind _keyvalue_9 (CallFunction|LoadData "eIncrease"))
      (CallFunction|AddMoney _keyvalue_9)))
  ;[1 1 1] Load and add to total earned
  (if (Variables|Default|GetonFirstRoom)
    (CallFunction|SaveData "pTotalEarned" (Utilities|Text|ToText(Float) (Variables|Default|GetearnedSubtotal) "HalfToEven" false false 1 324 2 2))
    (else
      (bind _keyvalue_10 (CallFunction|LoadData "pTotalEarned"))
      (CallFunction|SaveData "pTotalEarned" (Utilities|Text|ToText(Float) (+ _keyvalue_10 (Variables|Default|GetearnedSubtotal)) "HalfToEven" false false 1 324 2 2)))))

(event EventTick
  (params (DeltaSeconds :type Float%20%28single-precision%29))
  (bind _returnvalue (Game|GetPlayerController 0))
  (bind _hitresult (Game|Player|GetHitResultUnderCursorbyChannel _returnvalue "TraceTypeQuery1" true))
  (bind (_bblockinghit _binitialoverlap _time _distance _location _impactpoint _normal _impactnormal) (Collision|BreakHitResult _hitresult))
  ;[1 1 1] (Tick) Get position of Mouse in World* or Face Enemy
  (if (Variables|Default|GetinCombat)
    (CallFunction|FaceEnemy)
    (else
      (Transformation|SetWorldLocationAndRotation (Variables|Default|GetCursorToWorld) _location (Math|Rotator|MakeRotationfromAxes _impactnormal "0, 0, 0" "0, 0, 0") false false))))

(event Input|KeyboardEvents|Tab
  (params (Key :type Key%20Structure :default "None"))
  ;[1 0.3734 0] TEST open options menu
  (:Pressed
    (bind _returnvalue (UserInterface|CreateWidget "/Game/_FinanceRun/UI/fr_w_options.fr_w_options_C"))
    (UserInterface|Viewport|AddtoViewport _returnvalue 0)))

(fn ConstructionScript)

(fn SaveData
  (params (KeyName :type String) (KeyValue :type Text))
  ;[1 1 1] Save a value using EasySaveObject
  (bind _outactors (Actor|GetAllActorsOfClass "/Game/EasySave/easySaveObject.easySaveObject_C"))
  (for _array_element _outactors
    (bind _aseasy_save_object (Utilities|Casting|CastToeasySaveObject _array_element))
    (Default|EasySaveValue :self _aseasy_save_object :keyName KeyName :keyType "NewEnumerator1" :keyValue KeyValue)))

(fn LoadData
  (params (KeyName :type String))
  (bind _outactors (Actor|GetAllActorsOfClass "/Game/EasySave/easySaveObject.easySaveObject_C"))
  (for _array_element _outactors
    (bind _aseasy_save_object (Utilities|Casting|CastToeasySaveObject _array_element))
    (bind _valueasfloat (Default|EasyLoadValue _aseasy_save_object KeyName "NewEnumerator1" false))
    (return _valueasfloat)))

(fn StartCombat
  (params (Enemy :type Fr%20Bp%20Enemy%20Object%20Reference))
  ;[1 1 1] Set variable and change attributes to lock player into combat, create and add combat HUD
  (Variables|Default|SetenemyToFace Enemy)
  (Variables|Default|SetinCombat true)
  (Input|DisableInput 0)
  (Variables|/Script/Engine.CharacterMovementComponent|SetMaxWalkSpeed (Variables|Character|GetCharacterMovement) 0.0)
  (Rendering|SetVisibility (Variables|Default|GetCursorToWorld) false false)
  (bind _returnvalue (UserInterface|CreateWidget "/Game/_FinanceRun/UI/fr_w_combat.fr_w_combat_C"))
  (Variables|Default|SetcombatHUD _returnvalue)
  (Variables|/Game/_FinanceRun/UI/fr_w_combat.fr_w_combat_C|Setenemy _returnvalue (Variables|Default|GetenemyToFace))
  (UserInterface|Viewport|AddtoViewport _returnvalue 0)
  (Variables|/Game/_FinanceRun/Blueprints/Enemy/Core/fr_bp_enemy.fr_bp_enemy_C|SetCombatHUD (Variables|Default|GetenemyToFace) _returnvalue))

(fn FinishCombat
  (Game|Player|SetViewTargetwithBlend (Game|GetPlayerController 0) self 1.0 "VTBlend_Linear" 0.0 false)
  (Variables|Default|SetinCombat false)
  (Input|EnableInput 0)
  (Variables|/Script/Engine.CharacterMovementComponent|SetMaxWalkSpeed (Variables|Character|GetCharacterMovement) 6e+02)
  (Rendering|SetVisibility (Variables|Default|GetCursorToWorld) true false)
  (Widget|RemovefromParent (Variables|Default|GetcombatHUD)))